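; BP_ToxicEnemyComponent is a status component that keeps an enemy's toxic message in sync with its ToxicDMG status.
; It caches its owner as a BaseEnemy on BeginPlay.
; Each tick it polls the enemy for that status and passes its IsExploded flag to the owner's SwitchToxicMessage.
; When the status is no longer found, it switches the message to false and destroys itself.
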(event `self.ReceiveBeginPlay`
  (bind _asbase_enemy (cast `BaseEnemy` (`self.GetOwner`)))
  (set `self.Enemy` _asbase_enemy))

(event `self.ReceiveTick`
  (params (DeltaSeconds :type "Float (single-precision)"))
  (bind _returnvalue (message `StatusOwner.GetStatus` (`self.Enemy`) "ToxicDMG"))
  (bind _astoxic_dmg (cast `ToxicDMG` _returnvalue)
    (:`then`
      (message `/Game/Bluprints/Enemies/BPI_Enemy.SwitchToxic` (`self.GetOwner`) (`ExplodedStatus.IsExploded` _astoxic_dmg)))
    (:`CastFailed`
      (message `/Game/Bluprints/Enemies/BPI_Enemy.SwitchToxic` (`self.GetOwner`) false)
      (`self.K2_DestroyComponent`))))