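; Actor component that tracks the plasma damage status on an enemy and drives its feedback.
; On begin play it caches its owner as a BaseEnemy, then each tick polls that enemy for a PlasmaDMG status message.
; While the message is valid it keeps the plasma message switched on.
; Once it is gone, it switches the message off, spawns an attached plasma blast Niagara effect and destroys itself.
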(event `self.ReceiveBeginPlay`
  (bind _asbase_enemy (cast `BaseEnemy` (`self.GetOwner`)))
  (set `self.Enemy` _asbase_enemy))

(event `self.ReceiveTick`
  (params (DeltaSeconds :type "Float (single-precision)"))
  (bind _returnvalue (message `StatusOwner.GetStatus` (`self.Enemy`) "PlasmaDMG"))
  (`/Engine/EditorBlueprintResources/StandardMacros.IsValid` (`KismetSystemLibrary.Conv_InterfaceToObject` _returnvalue)
    (:`Is Valid`
      (message `/Game/Bluprints/Enemies/BPI_Enemy.SwitchPlasma` (`self.Enemy`) true))
    (:`Is Not Valid`
      (message `/Game/Bluprints/Enemies/BPI_Enemy.SwitchPlasma` (`self.Enemy`) false)
      (`NiagaraFunctionLibrary.SpawnSystemAttached` "/Game/Bluprints/Turrets/Particles/NS_PlasmaBlast.NS_PlasmaBlast" (`Actor.RootComponent` (`self.Enemy`)) "None" (0.0 0.0 0.0) (struct) "KeepRelativeOffset" true)
      (`self.K2_DestroyComponent`))))