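; Top-down camera actor that becomes the player's view target on BeginPlay and provides edge-scroll panning and zoom.
; Each tick, four move functions offset the spring arm along its relative X or Y axis when the mouse nears a viewport edge.
; Speed ramps linearly across a padding band, reaching full at the edge, without delta-time scaling.
; Zoom adjusts spring arm length from an input axis key, clamped between min and max distances.
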(event `self.ReceiveBeginPlay`
  (`PlayerController.SetViewTargetWithBlend` (`GameplayStatics.GetPlayerController` 0) self 0.0 "VTBlend_Linear" 0.0 false))

(event `self.ReceiveTick`
  (params (DeltaSeconds :type "Float (single-precision)"))
  (`self.MoveLeft`)
  (`self.MoveRight`)
  (`self.MoveUp`)
  (`self.MoveDown`)
  (`self.Zoom`))

(fn `MoveDown`
  (bind (_returnvalue_x _returnvalue_y) (`KismetMathLibrary.BreakVector2D` (`WidgetLayoutLibrary.GetViewportSize`)))
  (bind _returnvalue (`WidgetLayoutLibrary.GetMousePositionOnViewport`))
  (`SceneComponent.K2_AddRelativeLocation` (`self.SpringArm`) (* (* (-1.0 0.0 0.0) (`self.MoveSpeed`)) (`KismetMathLibrary.FClamp` (`KismetMathLibrary.NormalizeToRange` (`.Y` (`KismetMathLibrary.BreakVector2D` _returnvalue)) (* (- 1.0 (`self.Padding`)) _returnvalue_y) _returnvalue_y))) false false))

(fn `MoveLeft`
  (bind _returnvalue_x (`KismetMathLibrary.BreakVector2D` (`WidgetLayoutLibrary.GetViewportSize`)))
  (bind _returnvalue (`WidgetLayoutLibrary.GetMousePositionOnViewport`))
  (`SceneComponent.K2_AddRelativeLocation` (`self.SpringArm`) (* (* (0.0 -1.0 0.0) (`self.MoveSpeed`)) (- 1.0 (`KismetMathLibrary.FClamp` (`KismetMathLibrary.NormalizeToRange` (`KismetMathLibrary.BreakVector2D` _returnvalue) 0.0 (* _returnvalue_x (`self.Padding`)))))) false false))

(fn `MoveRight`
  (bind _returnvalue_x (`KismetMathLibrary.BreakVector2D` (`WidgetLayoutLibrary.GetViewportSize`)))
  (bind _returnvalue (`WidgetLayoutLibrary.GetMousePositionOnViewport`))
  (`SceneComponent.K2_AddRelativeLocation` (`self.SpringArm`) (* (* (0.0 1.0 0.0) (`self.MoveSpeed`)) (`KismetMathLibrary.FClamp` (`KismetMathLibrary.NormalizeToRange` (`KismetMathLibrary.BreakVector2D` _returnvalue) (* (- 1.0 (`self.Padding`)) _returnvalue_x) _returnvalue_x))) false false))

(fn `MoveUp`
  (bind (_returnvalue_x _returnvalue_y) (`KismetMathLibrary.BreakVector2D` (`WidgetLayoutLibrary.GetViewportSize`)))
  (bind _returnvalue (`WidgetLayoutLibrary.GetMousePositionOnViewport`))
  (`SceneComponent.K2_AddRelativeLocation` (`self.SpringArm`) (* (* (1.0 0.0 0.0) (`self.MoveSpeed`)) (- 1.0 (`KismetMathLibrary.FClamp` (`KismetMathLibrary.NormalizeToRange` (`.Y` (`KismetMathLibrary.BreakVector2D` _returnvalue)) 0.0 (* _returnvalue_y (`self.Padding`)))))) false false))

(fn `UserConstructionScript`)

(fn `Zoom`
  (set `SpringArmComponent.TargetArmLength` (`KismetMathLibrary.FClamp` (+ (* (`self.GetInputAxisKeyValue`) (* (`self.ZoomSpeed`) -1.0)) (`SpringArmComponent.TargetArmLength` (`self.SpringArm`))) (`self.MinDistance`) (`self.MaxDistance`)) (`self.SpringArm`)))