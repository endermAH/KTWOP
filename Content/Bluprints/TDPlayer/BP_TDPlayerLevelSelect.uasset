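; Level-select player pawn that takes over the view and lets the mouse pick a level to open.
; Each tick a cursor trace activates the hovered BP_Level_Point unless its state excludes it, and left click opens that level.
; Edge-scroll, zoom and bounded pan/rotate helpers exist but are not wired to Tick or input.
; Debug keys print the game instance's Souls and delete the main save slot.
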(event `self.ReceiveBeginPlay`
  (`PlayerController.SetViewTargetWithBlend` (`GameplayStatics.GetPlayerController` 0) self 0.0 "VTBlend_Linear" 0.0 false))

(event `self.ReceiveTick`
  (params (DeltaSeconds :type "Float (single-precision)"))
  (bind _asbp_level_point (cast `/Game/Bluprints/Map/Tiles/WorldMap/BP_Level_Point` (`.HitActor` (`GameplayStatics.BreakHitResult` (`PlayerController.GetHitResultUnderCursorByChannel` (`GameplayStatics.GetPlayerController` 0) "TraceTypeQuery4" true))))
    (:`then`
      (if (`|EnumInequality` (`/Game/Bluprints/Map/Tiles/WorldMap/BP_Level_Point.State` _asbp_level_point) "NewEnumerator1")
        (`/Game/Bluprints/Map/Tiles/WorldMap/BP_Level_Point.SetIsActive` _asbp_level_point true)
        (set `self.ActiveCoin` _asbp_level_point)))
    (:`CastFailed`
      (`/Engine/EditorBlueprintResources/StandardMacros.IsValid` (`self.ActiveCoin`)
        (:`Is Valid`
          (`/Game/Bluprints/Map/Tiles/WorldMap/BP_Level_Point.SetIsActive` (`self.ActiveCoin`) false)
          (set `self.ActiveCoin` null))))))

(event `InputAction|Cancel`
  (params (Key :type "Key Structure")))

(event `Key|LeftMouseButton`
  (params (Key :type "Key Structure"))
  (:`Pressed`
    (`/Engine/EditorBlueprintResources/StandardMacros.IsValid` (`self.ActiveCoin`)
      (:`Is Valid`
        (`/Game/Bluprints/Map/Tiles/WorldMap/BP_Level_Point.OpenLevel` (`self.ActiveCoin`))))))

(event `InputAxis|Horisontal`
  (params (AxisValue :type "Float (single-precision)")))

(event `Key|Zero`
  (params (Key :type "Key Structure"))
  (:`Pressed`
    (`KismetSystemLibrary.PrintString` (`KismetStringLibrary.Conv_IntToString` (`KTWOPGameInstance.Souls` (cast `/Game/Bluprints/Enemies/BP_KTWOPGameInstance` (`GameplayStatics.GetGameInstance`) :!pure true))))))

(event `InputAxis|Vertical`
  (params (AxisValue :type "Float (single-precision)")))

(event `Key|Nine`
  (params (Key :type "Key Structure"))
  (:`Pressed`
    (bind _returnvalue (`GameplayStatics.DeleteGameInSlot` "MAIN_SAVE"))
    (if _returnvalue
      (`KismetSystemLibrary.PrintString` "Deleted"))))

(event `InputAxis|Yaw`
  (params (AxisValue :type "Float (single-precision)")))

(fn `Move Right with Cursor`
  (bind _returnvalue_x (`KismetMathLibrary.BreakVector2D` (`WidgetLayoutLibrary.GetViewportSize`)))
  (bind _returnvalue (/ _returnvalue_x (`WidgetLayoutLibrary.GetViewportScale`)))
  (bind _returnvalue_2 (`WidgetLayoutLibrary.GetMousePositionOnViewport`))
  (`self.Update Position` (* (`KismetMathLibrary.GreaterGreater_VectorRotator` (`KismetMathLibrary.MakeVector` 0.0 1.0) (`SceneComponent.RelativeRotation` (`self.Point`))) (`KismetMathLibrary.FClamp` (`KismetMathLibrary.NormalizeToRange` (`KismetMathLibrary.BreakVector2D` _returnvalue_2) (* (- 1.0 (`self.Padding`)) _returnvalue) _returnvalue)))))

(fn `Move with Cursor`
  (`self.MoveLeftWithCursor`)
  (`self.Move Right with Cursor`)
  (`self.MoveUpWithCursor`)
  (`self.MoveDownWithCursor`)
  (`self.Zoom`))

(fn `MoveDownWithCursor`
  (bind (_returnvalue_x _returnvalue_y) (`KismetMathLibrary.BreakVector2D` (`WidgetLayoutLibrary.GetViewportSize`)))
  (bind _returnvalue (/ _returnvalue_y (`WidgetLayoutLibrary.GetViewportScale`)))
  (bind _returnvalue_2 (`WidgetLayoutLibrary.GetMousePositionOnViewport`))
  (`self.Update Position` (* (`KismetMathLibrary.GreaterGreater_VectorRotator` (`KismetMathLibrary.MakeVector` -1.0) (`SceneComponent.RelativeRotation` (`self.Point`))) (`KismetMathLibrary.FClamp` (`KismetMathLibrary.NormalizeToRange` (`.Y` (`KismetMathLibrary.BreakVector2D` _returnvalue_2)) (* (- 1.0 (`self.Padding`)) _returnvalue) _returnvalue)))))

(fn `MoveLeftWithCursor`
  (bind _returnvalue_x (`KismetMathLibrary.BreakVector2D` (`WidgetLayoutLibrary.GetViewportSize`)))
  (bind _returnvalue (`WidgetLayoutLibrary.GetMousePositionOnViewport`))
  (`self.Update Position` (* (`KismetMathLibrary.GreaterGreater_VectorRotator` (`KismetMathLibrary.MakeVector` 0.0 -1.0) (`SceneComponent.RelativeRotation` (`self.Point`))) (- 1.0 (`KismetMathLibrary.FClamp` (`KismetMathLibrary.NormalizeToRange` (`KismetMathLibrary.BreakVector2D` _returnvalue) 0.0 (* (/ _returnvalue_x (`WidgetLayoutLibrary.GetViewportScale`)) (`self.Padding`))))))))

(fn `MoveUpWithCursor`
  (bind (_returnvalue_x _returnvalue_y) (`KismetMathLibrary.BreakVector2D` (`WidgetLayoutLibrary.GetViewportSize`)))
  (bind _returnvalue (`WidgetLayoutLibrary.GetMousePositionOnViewport`))
  (`self.Update Position` (* (`KismetMathLibrary.GreaterGreater_VectorRotator` (`KismetMathLibrary.MakeVector` 1.0) (`SceneComponent.RelativeRotation` (`self.Point`))) (- 1.0 (`KismetMathLibrary.FClamp` (`KismetMathLibrary.NormalizeToRange` (`.Y` (`KismetMathLibrary.BreakVector2D` _returnvalue)) 0.0 (* (/ _returnvalue_y (`WidgetLayoutLibrary.GetViewportScale`)) (`self.Padding`))))))))

(fn `Update`)

(fn `Update Position`
  (params (DeltaPosition :type "Vector Structure"))
  (bind (_minx _maxx _miny _maxy) (`self.Bounds`))
  (bind (_returnvalue_x _returnvalue_y) (`KismetMathLibrary.BreakVector` (+ (* (`KismetMathLibrary.Normal` DeltaPosition) (`self.MoveSpeed`)) (`SceneComponent.RelativeLocation` (`self.Point`)))))
  (`SceneComponent.K2_SetRelativeLocation` (`self.Point`) (`KismetMathLibrary.MakeVector` (`KismetMathLibrary.FClamp` _returnvalue_x _minx _maxx) (`KismetMathLibrary.FClamp` _returnvalue_y _miny _maxy)) false false))

(fn `UpdateRotation`
  (params (DeltaAngle :type "Float (double-precision)"))
  (`SceneComponent.K2_AddRelativeRotation` (`self.Point`) (`KismetMathLibrary.MakeRotator` 0.0 0.0 DeltaAngle) false false))

(fn `UserConstructionScript`
  (`SceneComponent.SetWorldScale3D` (`self.Box`) (`KismetMathLibrary.MakeVector` (`self.ScaleX`) (`self.ScaleY`) (`self.ScaleZ`))))

(fn `Zoom`
  (set `SpringArmComponent.TargetArmLength` (`KismetMathLibrary.FClamp` (+ (* (`self.GetInputAxisKeyValue`) (* (`self.ZoomSpeed`) -1.0)) (`SpringArmComponent.TargetArmLength` (`self.SpringArm`))) (`self.MinDistance`) (`self.MaxDistance`)) (`self.SpringArm`)))