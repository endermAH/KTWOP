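; Player controller, likely for a top-down player, that on BeginPlay sets Game and UI input with the mouse always locked and the cursor visible during capture.
; Helper functions move the controlled pawn along the control rotation's forward and right vectors.
; The movement and mouse axis events are empty, so those helpers and the cursor-repositioning logic sit disconnected and never run.
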(event `self.ReceiveBeginPlay`
  (`WidgetBlueprintLibrary.SetInputMode_GameAndUIEx` self null "LockAlways" false))

(event `InputAxis|Vertical`
  (params (AxisValue :type "Float (single-precision)")))

(event `InputAxis|Horisontal`
  (params (AxisValue :type "Float (single-precision)")))

(event `Key|LeftMouseButton`
  (params (Key :type "Key Structure")))

(event `InputAxisKey|MouseY`
  (params (AxisValue :type "Float (single-precision)")))

(event `InputAxisKey|MouseX`
  (params (AxisValue :type "Float (single-precision)")))

(fn `ApplyHorisontalInput`
  (params (Scale :type "Float (double-precision)"))
  (`Pawn.AddMovementInput` (`self.K2_GetPawn`) (`KismetMathLibrary.GetRightVector` (`self.GetControlRotation`)) (`local.Scale`) false))

(fn `ApplyVerticalInput`
  (params (Scale :type "Float (double-precision)"))
  (`Pawn.AddMovementInput` (`self.K2_GetPawn`) (`KismetMathLibrary.GetForwardVector` (`self.GetControlRotation`)) (`local.Scale`) false))

(fn `UserConstructionScript`)