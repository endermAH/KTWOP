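; Tower-defense player: a bounded RTS-style camera that also handles turret placement and the tower-button HUD.
; Axis input and screen-edge cursor scrolling move the Point within Box bounds, with yaw rotation and spring-arm zoom.
; Cannon and laser buttons check GameInstance stones, then enter a Phantom state where a preview follows hovered tiles, left click attempts spawning and Cancel clears it.
; The third tower button's handler is empty.
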(event `self.ReceiveBeginPlay`
  (`PlayerController.SetViewTargetWithBlend` (`GameplayStatics.GetPlayerController` 0) self 0.0 "VTBlend_Linear" 0.0 false)
  (bind _interface (`self.SetupInterface`))
  (set `self.UI` _interface))

(event `self.ReceiveTick`
  (params (DeltaSeconds :type "Float (single-precision)"))
  (`self.Move with Cursor`)
  (`self.Update`)
  (bind _asbp_ktwopgame_instance (cast `/Game/Bluprints/Enemies/BP_KTWOPGameInstance` (`GameplayStatics.GetGameInstance`)))
  (`/Game/UI/W_Hub.ChangeStouneCount` (`self.UI`) (`KTWOPGameInstance.Stones` _asbp_ktwopgame_instance)))

(event `InputAction|Cancel`
  (params (Key :type "Key Structure"))
  (:`Pressed`
    (`self.Reset`)))

(event `Key|LeftMouseButton`
  (params (Key :type "Key Structure"))
  (:`Pressed`
    (`self.Act`)))

(event `InputAxis|Horisontal`
  (params (AxisValue :type "Float (single-precision)"))
  (`self.UpdatePosition` (* (`SceneComponent.GetForwardVector` (`self.Point`)) (* AxisValue (`self.MoveSpeed`)))))

(event `InputAxis|Vertical`
  (params (AxisValue :type "Float (single-precision)"))
  (`self.UpdatePosition` (* (`SceneComponent.GetRightVector` (`self.Point`)) (* AxisValue (`self.MoveSpeed`)))))

(event `InputAxis|Yaw`
  (params (AxisValue :type "Float (single-precision)"))
  (`self.UpdateRotation` (* AxisValue (`self.RotationSpeed`))))

(fn `Act`
  (switch `/Game/Bluprints/TDPlayer/E_TDPlayerState` (`self.State`)
    (:`NewEnumerator1`
      (bind _asbp_tile (cast `/Game/Bluprints/Map/Tiles/BP_Tile` (`.HitActor` (`GameplayStatics.BreakHitResult` (`PlayerController.GetHitResultUnderCursorByChannel` (`GameplayStatics.GetPlayerController` 0) "TraceTypeQuery3" true)))))
      (`/Game/Bluprints/Phantom/BP_Phantom.TrySpawn` (`self.Phantom`) _asbp_tile))))

(fn `HasEnoughStones`
  (returns (NewParam :type Boolean))
  (bind _stones (`KTWOPGameInstance.Stones` (cast `/Game/Bluprints/Enemies/BP_KTWOPGameInstance` (`GameplayStatics.GetGameInstance`) :!pure true)))
  (`KismetSystemLibrary.PrintString` (`KismetStringLibrary.Concat_StrStr` "Net monet: " (`KismetStringLibrary.Conv_IntToString` _stones)))
  (return (>= _stones 100)))

(fn `Move Right with Cursor`
  (bind _returnvalue_x (`KismetMathLibrary.BreakVector2D` (`WidgetLayoutLibrary.GetViewportSize`)))
  (bind _returnvalue (`WidgetLayoutLibrary.GetMousePositionOnViewport`))
  (`self.UpdatePosition` (* (* (* (`SceneComponent.GetForwardVector` (`self.Point`)) -1.0) (`self.MoveSpeed`)) (`KismetMathLibrary.FClamp` (`KismetMathLibrary.NormalizeToRange` (`KismetMathLibrary.BreakVector2D` _returnvalue) (* (- 1.0 (`self.Padding`)) _returnvalue_x) _returnvalue_x)))))

(fn `Move with Cursor`
  (`self.MoveLeftWithCursor`)
  (`self.Move Right with Cursor`)
  (`self.MoveUpWithCursor`)
  (`self.MoveDownWithCursor`)
  (`self.Zoom`))

(fn `MoveDownWithCursor`
  (bind (_returnvalue_x _returnvalue_y) (`KismetMathLibrary.BreakVector2D` (`WidgetLayoutLibrary.GetViewportSize`)))
  (bind _returnvalue (`WidgetLayoutLibrary.GetMousePositionOnViewport`))
  (`self.UpdatePosition` (* (* (* (`SceneComponent.GetRightVector` (`self.Point`)) -1.0) (`self.MoveSpeed`)) (`KismetMathLibrary.FClamp` (`KismetMathLibrary.NormalizeToRange` (`.Y` (`KismetMathLibrary.BreakVector2D` _returnvalue)) (* (- 1.0 (`self.Padding`)) _returnvalue_y) _returnvalue_y)))))

(fn `MoveLeftWithCursor`
  (bind _returnvalue_x (`KismetMathLibrary.BreakVector2D` (`WidgetLayoutLibrary.GetViewportSize`)))
  (bind _returnvalue (`WidgetLayoutLibrary.GetMousePositionOnViewport`))
  (`self.UpdatePosition` (* (* (`SceneComponent.GetForwardVector` (`self.Point`)) (`self.MoveSpeed`)) (- 1.0 (`KismetMathLibrary.FClamp` (`KismetMathLibrary.NormalizeToRange` (`KismetMathLibrary.BreakVector2D` _returnvalue) 0.0 (* _returnvalue_x (`self.Padding`))))))))

(fn `MoveUpWithCursor`
  (bind (_returnvalue_x _returnvalue_y) (`KismetMathLibrary.BreakVector2D` (`WidgetLayoutLibrary.GetViewportSize`)))
  (bind _returnvalue (`WidgetLayoutLibrary.GetMousePositionOnViewport`))
  (`self.UpdatePosition` (* (* (`SceneComponent.GetRightVector` (`self.Point`)) (`self.MoveSpeed`)) (- 1.0 (`KismetMathLibrary.FClamp` (`KismetMathLibrary.NormalizeToRange` (`.Y` (`KismetMathLibrary.BreakVector2D` _returnvalue)) 0.0 (* _returnvalue_y (`self.Padding`))))))))

(fn `OnTurret1Clicked`
  (if (`self.HasEnoughStones`)
    (`self.SwitchToPhantom` "/Game/Bluprints/Phantom/BP_CannonPhantom.BP_CannonPhantom_C")))

(fn `OnTurret2Clicked`
  (if (`self.HasEnoughStones`)
    (`self.SwitchToPhantom` "/Game/Bluprints/Phantom/BP_LaserPhantom.BP_LaserPhantom_C")))

(fn `OnTurret3Clicked`)

(fn `Reset`
  (switch `/Game/Bluprints/TDPlayer/E_TDPlayerState` (`self.State`)
    (:`NewEnumerator1`
      (`self.K2_DestroyActor` (`self.Phantom`))
      (set `self.Phantom` null)
      (set `self.State` "NewEnumerator0"))))

(fn `SetupInterface`
  (returns (Interface :type "/Game/UI/W_Hub Object Reference"))
  (locals (Hub :type "/Game/UI/W_Hub Object Reference"))
  (bind _returnvalue (`|CreateWidget` "/Game/UI/W_Hub.W_Hub_C"))
  (set `local.Hub` _returnvalue)
  (`UserWidget.AddToViewport` (`local.Hub`) 0)
  (`|ExecutionSequence`
    (:`then_0`
      (bind _returnvalue_2 (`|CreateWidget` "/Game/UI/W_Tower.W_Tower_C" null 100.0 "/Game/UI/Images/TowerIcons/I_WeaponCanon.I_WeaponCanon"))
      (add `/Game/UI/W_Tower.OnClick` _returnvalue_2 (`|CreateDelegate` :!event `OnTurret1Clicked`))
      (`/Game/UI/W_Hub.AddTowerButton` (`local.Hub`) _returnvalue_2))
    (:`then_1`
      (bind _returnvalue_3 (`|CreateWidget` "/Game/UI/W_Tower.W_Tower_C" null 100.0 "/Game/UI/Images/TowerIcons/I_WeaponLazer.I_WeaponLazer"))
      (add `/Game/UI/W_Tower.OnClick` _returnvalue_3 (`|CreateDelegate` :!event `OnTurret2Clicked`))
      (`/Game/UI/W_Hub.AddTowerButton` (`local.Hub`) _returnvalue_3))
    (:`then_2`
      (bind _returnvalue_4 (`|CreateWidget` "/Game/UI/W_Tower.W_Tower_C" null 100.0 "/Game/UI/Images/TowerIcons/I_WeaponVapeMachine.I_WeaponVapeMachine"))
      (add `/Game/UI/W_Tower.OnClick` _returnvalue_4 (`|CreateDelegate` :!event `OnTurret3Clicked`))
      (`/Game/UI/W_Hub.AddTowerButton` (`local.Hub`) _returnvalue_4))
    (:`then_3`
      (return (`local.Hub`)))))

(fn `SwitchToPhantom`
  (params (Phantom :type "/Game/Bluprints/Phantom/BP_Phantom Class Reference"))
  (`self.Reset`)
  (bind _returnvalue (`|SpawnActorFromClass` (`local.Phantom`) (`KismetMathLibrary.MakeTransform` (`self.K2_GetActorLocation`)) "Undefined" "OverrideRootScale" null null))
  (set `self.Phantom` _returnvalue)
  (set `self.State` "NewEnumerator1"))

(fn `Update`
  (switch `/Game/Bluprints/TDPlayer/E_TDPlayerState` (`self.State`)
    (:`NewEnumerator1`
      (`self.Update Phantom`))))

(fn `Update Phantom`
  (bind _asbp_tile (cast `/Game/Bluprints/Map/Tiles/BP_Tile` (`.HitActor` (`GameplayStatics.BreakHitResult` (`PlayerController.GetHitResultUnderCursorByChannel` (`GameplayStatics.GetPlayerController` 0) "TraceTypeQuery3" true)))))
  (`/Engine/EditorBlueprintResources/StandardMacros.IsValid` (`self.Phantom`)
    (:`Is Valid`
      (bind _position (`/Game/Bluprints/Map/Tiles/BP_Tile.GetSocketPosition` _asbp_tile))
      (`self.K2_SetActorLocation` (`self.Phantom`) _position false false)
      (`/Game/Bluprints/Phantom/BP_Phantom.Update` (`self.Phantom`) _asbp_tile))))

(fn `UpdatePosition`
  (params (DeltaPosition :type "Vector Structure"))
  (bind (_minx _maxx _miny _maxy) (`self.Bounds`))
  (bind (_returnvalue_x _returnvalue_y) (`KismetMathLibrary.BreakVector` (+ DeltaPosition (`SceneComponent.RelativeLocation` (`self.Point`)))))
  (`SceneComponent.K2_SetRelativeLocation` (`self.Point`) (`KismetMathLibrary.MakeVector` (`KismetMathLibrary.FClamp` _returnvalue_x _minx _maxx) (`KismetMathLibrary.FClamp` _returnvalue_y _miny _maxy)) false false))

(fn `UpdateRotation`
  (params (DeltaAngle :type "Float (double-precision)"))
  (`SceneComponent.K2_AddRelativeRotation` (`self.Point`) (`KismetMathLibrary.MakeRotator` 0.0 0.0 DeltaAngle) false false))

(fn `UserConstructionScript`
  (`SceneComponent.SetWorldScale3D` (`self.Box`) (`KismetMathLibrary.MakeVector` (`self.ScaleX`) (`self.ScaleY`) (`self.ScaleZ`))))

(fn `Zoom`
  (set `SpringArmComponent.TargetArmLength` (`KismetMathLibrary.FClamp` (+ (* (`self.GetInputAxisKeyValue`) (* (`self.ZoomSpeed`) -1.0)) (`SpringArmComponent.TargetArmLength` (`self.SpringArm`))) (`self.MinDistance`) (`self.MaxDistance`)) (`self.SpringArm`)))