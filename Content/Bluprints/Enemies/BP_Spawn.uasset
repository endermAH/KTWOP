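; BP_Spawn is an enemy spawner that releases a limited Count of EnemyType actors, handing each its Aim.
; The construction script moves Point, the spawn location, to the socket of the tile found beneath the actor.
; BeginPlay hides the Widget and activates spawning after InitialDelay; Reset deactivates it.
; While active with Count remaining, Tick runs through a Delay that paces each spawn, which decrements Count.
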(event `self.ReceiveBeginPlay`
  (`SceneComponent.SetVisibility` (`self.Widget`) false false)
  (`KismetSystemLibrary.Delay` (`self.InitialDelay`))
  (set `self.IsActive` true))

(event `Reset`
  (set `self.IsActive` false))

(event `self.ReceiveTick`
  (params (DeltaSeconds :type "Float (single-precision)"))
  (if (`self.IsActive`)
    (if (> (`self.Count`) 0)
      (`KismetSystemLibrary.Delay` (`self.Delay`))
      (`self.SpawnEnamy`))))

(fn `SpawnEnamy`
  (locals (Enemy :type "/Game/Bluprints/Enemies/BP_BaseEnemy Object Reference"))
  (bind _returnvalue (`|SpawnActorFromClass` (`self.EnemyType`) (`KismetMathLibrary.MakeTransform` (`SceneComponent.K2_GetComponentLocation` (`self.Point`))) "Undefined" "OverrideRootScale" null null))
  (set `local.Enemy` _returnvalue)
  (set `/Game/Bluprints/Enemies/BP_BaseEnemy.Aim` (`self.Aim`) (`local.Enemy`))
  (`/Engine/EditorBlueprintResources/StandardMacros.DecrementInt` (`self.Count`)))

(fn `UserConstructionScript`
  (bind _tile (`/Game/Bluprints/Map/Utils/BP_MapUtils.Get Undertile` (`self.K2_GetActorLocation`) 100.0))
  (bind _position (`/Game/Bluprints/Map/Tiles/BP_Tile.GetSocketPosition` _tile))
  (`SceneComponent.K2_SetWorldLocation` (`self.Point`) _position false false))