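; BP_KTWOPGameInstance is the game instance that saves and loads the player's Souls and LevelsState.
; SaveGame creates a fresh BP_SaveGame object, copies both values into it and writes it to the fixed MAIN_SAVE slot.
; LoadGame reads that slot and restores both values, or prints "Nothing saved" when the cast to BP_SaveGame fails.
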(fn `LoadGame`
  (bind _returnvalue (`GameplayStatics.LoadGameFromSlot` "MAIN_SAVE"))
  (bind _asbp_save_game (cast `/Game/Bluprints/BP_SaveGame` _returnvalue)
    (:`then`
      (set `self.LevelsState` (`/Game/Bluprints/BP_SaveGame.LevelsState` _asbp_save_game))
      (set `self.Souls` (`/Game/Bluprints/BP_SaveGame.Souls` _asbp_save_game)))
    (:`CastFailed`
      (`KismetSystemLibrary.PrintString` "Nothing saved"))))

(fn `SaveGame`
  (locals (SaveObject :type "/Game/Bluprints/BP_SaveGame Object Reference"))
  (bind _returnvalue (`GameplayStatics.CreateSaveGameObject` "/Game/Bluprints/BP_SaveGame.BP_SaveGame_C"))
  (bind _output_get (set `local.SaveObject` _returnvalue))
  (set `/Game/Bluprints/BP_SaveGame.Souls` (`self.Souls`) _output_get)
  (set `/Game/Bluprints/BP_SaveGame.LevelsState` (`self.LevelsState`) (`local.SaveObject`))
  (`GameplayStatics.SaveGameToSlot` (`local.SaveObject`) "MAIN_SAVE"))