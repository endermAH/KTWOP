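; BP_Aim is the target that enemies damage on contact, with its own Hp that ends the game when depleted.
; An enemy entering its Sphere subtracts its AimDamage from Hp and is destroyed; Hp is printed, and at zero or below the MainMenu level opens.
; The construction script finds the tile beneath the actor and moves the Point component to that tile's socket position.
; Its Widget is hidden on BeginPlay.
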(event `self.ReceiveBeginPlay`
  (`SceneComponent.SetVisibility` (`self.Widget`) false false))

(event `self.ReceiveActorBeginOverlap`
  (params (OtherActor :type "Actor Object Reference")))

(event `self.ReceiveTick`
  (params (DeltaSeconds :type "Float (single-precision)")))

(event `self.Sphere.OnComponentBeginOverlap`
  (params (OverlappedComponent :type "PrimitiveComponent Object Reference") (OtherActor :type "Actor Object Reference") (OtherComp :type "PrimitiveComponent Object Reference") (OtherBodyIndex :type Integer) (bFromSweep :type Boolean) (SweepResult :type "HitResult Structure (by ref)"))
  (bind _asbp_base_enemy (cast `/Game/Bluprints/Enemies/BP_BaseEnemy` OtherActor))
  (bind _output_get (set `self.hp` (- (`self.hp`) (`/Game/Bluprints/Enemies/BP_BaseEnemy.aim_damage` _asbp_base_enemy))))
  (`KismetSystemLibrary.PrintString` (`KismetStringLibrary.Conv_IntToString` _output_get))
  (`self.K2_DestroyActor` _asbp_base_enemy)
  (if (<= (`self.hp`) 0)
    (`GameplayStatics.OpenLevelBySoftObjectPtr` "/Game/Maps/GameLoop/MainMenu.MainMenu")))

(fn `UserConstructionScript`
  (bind _tile (`/Game/Bluprints/Map/Utils/BP_MapUtils.Get Undertile` (`self.K2_GetActorLocation`) 100.0))
  (`/Engine/EditorBlueprintResources/StandardMacros.IsValid` _tile
    (:`Is Valid`
      (bind _position (`/Game/Bluprints/Map/Tiles/BP_BaseTile.GetSocketPosition` _tile))
      (`SceneComponent.K2_SetWorldLocation` (`self.Point`) _position false false))))