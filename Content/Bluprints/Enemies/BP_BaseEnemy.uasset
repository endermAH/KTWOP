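; BP_BaseEnemy is the base enemy Blueprint, handling health display, status-effect visuals and death rewards.
; A dark red widget HP bar follows EnemyStats health every Tick and hides at full health.
; On death it destroys itself, adds stone and soul rewards to the game instance, and notifies BP_Aim.
; Switch events toggle toxic, ice and plasma visuals, while damage and currency totals print to screen.
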(event `self.ReceiveBeginPlay`
  (bind _asbpw_hpbar (cast `/Game/Bluprints/Enemies/UI/BPW_HPBar` (`WidgetComponent.GetWidget` (`self.Widget`))))
  (bind _output_get (set `self.HPBar` _asbpw_hpbar))
  (set `/Game/Bluprints/Enemies/UI/BPW_HPBar.Color` (struct :`R` 0.359375 :`A` 1.0) _output_get))

(event `self.ReceiveTick`
  (params (DeltaSeconds :type "Float (single-precision)"))
  (bind (_enemystats_maxhealth _enemystats_collisionradius _enemystats_health) (break `EnemyStats` (`self.EnemyStats`)))
  (bind _hpbar (`self.HPBar`))
  (set `/Game/Bluprints/Enemies/UI/BPW_HPBar.HP` (/ _enemystats_health _enemystats_maxhealth) _hpbar)
  (if (== _enemystats_health _enemystats_maxhealth)
    (`Widget.SetVisibility` _hpbar "Hidden")
    (else
      (`Widget.SetVisibility` _hpbar "Visible"))))

(event `self.OnDeath`
  (bind _asbp_ktwopgame_instance (cast `/Game/Bluprints/Enemies/BP_KTWOPGameInstance` (`GameplayStatics.GetGameInstance`) :!pure true))
  (`self.K2_DestroyActor`)
  (`KTWOPGameInstance.IncreaseStones` _asbp_ktwopgame_instance (`self.stone_cost`))
  (`KTWOPGameInstance.IncreaseSouls` _asbp_ktwopgame_instance (`self.soul_cost`))
  (`KismetSystemLibrary.PrintString` (`KismetStringLibrary.Concat_StrStr` "Stones:" (`KismetStringLibrary.Conv_IntToString` (`KTWOPGameInstance.Stones` _asbp_ktwopgame_instance)) " \n" "Souls: " (`KismetStringLibrary.Conv_IntToString` (`KTWOPGameInstance.Souls` _asbp_ktwopgame_instance))))
  (bind _returnvalue (`GameplayStatics.GetActorOfClass` "/Game/Bluprints/Enemies/BP_Aim.BP_Aim_C"))
  (`/Game/Bluprints/Enemies/BP_Aim.EnemyDefeated` _returnvalue))

(event `self.ShowApplyedDamage`
  (params (damage :type "Float (single-precision)"))
  (`KismetSystemLibrary.PrintString` (`KismetStringLibrary.Conv_DoubleToString` damage)))

(event `/Game/Bluprints/Enemies/BPI_Enemy.SwitchToxic`
  (params (IsOn :type Boolean))
  (`SceneComponent.SetVisibility` (`self.Toxic`) IsOn false))

(event `/Game/Bluprints/Enemies/BPI_Enemy.SwitchIce`
  (params (IsOn :type Boolean))
  (for _array_element (`|MakeArray` (`self.Body`) (`self.BackLeftLeg`) (`self.FrontRightLeg`) (`self.FrontLeftLeg`) (`self.BackRightLeg`))
    (`SceneComponent.SetVisibility` _array_element IsOn false)))

(event `/Game/Bluprints/Enemies/BPI_Enemy.SwitchPlasma`
  (params (IsOn :type Boolean))
  (`SceneComponent.SetVisibility` (`self.Plasma`) IsOn false))

(fn `UserConstructionScript`)