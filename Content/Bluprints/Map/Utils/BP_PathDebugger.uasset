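; Debug actor that visualizes the tile path BP_Map finds between its Start and Finish components.
; FindPath clears old markers, gets BP_Map, resolves the tile under each endpoint via GetUndertile, then calls the map's FindPathBetweenTiles.
; Each returned location becomes a small instanced static mesh, while a missing map or tile prints a message.
; Nothing runs on play or construction, so FindPath and Clear must be invoked explicitly.
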(event `self.ReceiveBeginPlay`)

(fn `Clear`
  (`InstancedStaticMeshComponent.ClearInstances` (`self.InstancedStaticMesh`)))

(fn `Find Path`
  (locals (Map :type "/Game/Bluprints/Map/BP_Map Object Reference") (StartTile :type "/Game/Bluprints/Map/Tiles/BP_Tile Object Reference") (EndTile :type "/Game/Bluprints/Map/Tiles/BP_Tile Object Reference"))
  (`self.Clear`)
  (bind _returnvalue (`GameplayStatics.GetActorOfClass` "/Game/Bluprints/Map/BP_Map.BP_Map_C"))
  (`/Engine/EditorBlueprintResources/StandardMacros.IsValid` _returnvalue
    (:`Is Valid`
      (set `local.Map` _returnvalue)
      (bind _tile (`/Game/Bluprints/Map/Utils/BP_MapUtils.Get Undertile` self (`SceneComponent.K2_GetComponentLocation` (`self.Start`)) 100.0))
      (`/Engine/EditorBlueprintResources/StandardMacros.IsValid` _tile
        (:`Is Valid`
          (set `local.StartTile` _tile)
          (bind _tile_2 (`/Game/Bluprints/Map/Utils/BP_MapUtils.Get Undertile` self (`SceneComponent.K2_GetComponentLocation` (`self.Finish`)) 100.0))
          (`/Engine/EditorBlueprintResources/StandardMacros.IsValid` _tile_2
            (:`Is Valid`
              (set `local.EndTile` _tile_2)
              (bind _path (`/Game/Bluprints/Map/BP_Map.FindPathBetweenTiles` (`local.Map`) (`local.StartTile`) (`local.EndTile`)))
              (for _array_element _path
                (`InstancedStaticMeshComponent.AddInstanceWorldSpace` (`self.InstancedStaticMesh`) (`KismetMathLibrary.MakeTransform` _array_element (struct) (0.1 0.1 0.1)))))
            (:`Is Not Valid`
              (`KismetSystemLibrary.PrintString` "To is none"))))
        (:`Is Not Valid`
          (`KismetSystemLibrary.PrintString` "From is none"))))
    (:`Is Not Valid`
      (`KismetSystemLibrary.PrintString` "Map isn't founded"))))

(fn `UserConstructionScript`)