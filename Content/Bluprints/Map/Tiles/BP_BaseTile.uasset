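; BP_BaseTile is the base map tile, registering with BP_Map and offering a socket position plus one attachable reference.
; Its construction script removes the tile from the map, runs the anchor component's construction logic, then re-adds it.
; Swap uses chained timelines to sink the mesh, unregister, spawn another tile type in place and raise it.
; The old tile then destroys itself but passes itself, not the spawned tile, to AddTile.
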(event `Swap`
  (params (TileType :type "/Game/Bluprints/Map/Tiles/BP_BaseTile Class Reference"))
  (bind (_returnvalue_location _returnvalue_rotation) (`KismetMathLibrary.BreakTransform` (`self.GetTransform` self)))
  (bind (_direction _newtrack_0) (`Timeline|Move` :`NewTime` 10.0 :!via `PlayFromStart`)
    (:`Update`
      (`SceneComponent.K2_SetRelativeLocation` (`self.Mesh`) (`KismetMathLibrary.MakeVector` 0.0 0.0 (`KismetMathLibrary.Lerp` 0.0 -200.0 _newtrack_0)) false false))
    (:`Finished`
      (bind _returnvalue (`GameplayStatics.GetActorOfClass` "/Game/Bluprints/Map/BP_Map.BP_Map_C"))
      (`/Game/Bluprints/Map/BP_Map.RemoveTile` _returnvalue self)
      (bind _returnvalue_2 (`|SpawnActorFromClass` TileType (`KismetMathLibrary.MakeTransform` _returnvalue_location _returnvalue_rotation) "Undefined" "OverrideRootScale" null null))
      (bind _mesh (`/Game/Bluprints/Map/Tiles/BP_BaseTile.Mesh` _returnvalue_2))
      (`SceneComponent.K2_SetRelativeLocation` _mesh (0.0 0.0 -200.0) false false)
      (bind (_direction_2 _z) (`Timeline|Timeline_0` :!via `PlayFromStart`)
        (:`Update`
          (`SceneComponent.K2_SetRelativeLocation` _mesh (`KismetMathLibrary.MakeVector` 0.0 0.0 (`KismetMathLibrary.Lerp` -200.0 0.0 _z)) false false))
        (:`Finished`
          (`self.K2_DestroyActor`)
          (`/Game/Bluprints/Map/BP_Map.AddTile` _returnvalue self))))))

(fn `AddTileToMap`
  (params (Map :type "/Game/Bluprints/Map/BP_Map Object Reference"))
  (`/Game/Bluprints/Map/BP_Map.AddTile` Map self))

(fn `Attach`
  (params (Attached :type "BaseTurret Object Reference"))
  (set `self.Attached` Attached))

(fn `DeleteFromEditor`
  (bind _returnvalue (`GameplayStatics.GetActorOfClass` "/Game/Bluprints/Map/BP_Map.BP_Map_C"))
  (`/Engine/EditorBlueprintResources/StandardMacros.IsValid` _returnvalue
    (:`Is Valid`
      (`/Game/Bluprints/Map/BP_Map.RemoveTile` _returnvalue self)
      (`self.K2_DestroyActor`))))

(fn `Detach`
  (returns (Detached :type "Actor Object Reference"))
  (locals (Temp :type "Actor Object Reference"))
  (set `local.Temp` (`self.Attached`))
  (set `self.Attached` null)
  (return (`local.Temp`)))

(fn `GetAttached`
  (returns (Attached :type "BaseTurret Object Reference"))
  (return (`self.Attached`)))

(fn `GetPosition`
  (returns (Position :type "Vector Structure"))
  (return (`SceneComponent.K2_GetComponentLocation` (`self.Mesh`))))

(fn `GetSocketPosition`
  (returns (Position :type "Vector Structure"))
  (return (`SceneComponent.K2_GetComponentLocation` (`self.Socket`))))

(fn `IsHasAttached`
  (returns (IsHasAttached :type Boolean))
  (return (`KismetSystemLibrary.IsValid` (`self.Attached`))))

(fn `RemoveTileFromMap`
  (params (Map :type "/Game/Bluprints/Map/BP_Map Object Reference"))
  (`/Game/Bluprints/Map/BP_Map.RemoveTile` Map self))

(fn `UserConstructionScript`
  (bind _returnvalue (`GameplayStatics.GetActorOfClass` "/Game/Bluprints/Map/BP_Map.BP_Map_C"))
  (`/Engine/EditorBlueprintResources/StandardMacros.IsValid` _returnvalue
    (:`Is Valid`
      (`self.RemoveTileFromMap` _returnvalue)
      (`/Game/Bluprints/Map/BP_MapAnchorComponent.ExternaConstructionScript` (`self.BP_MapAnchorComponent`))
      (`self.AddTileToMap` _returnvalue))))