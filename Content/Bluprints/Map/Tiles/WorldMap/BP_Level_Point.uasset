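; BP_Level_Point is a world map marker for one level, showing its number, section and availability.
; On BeginPlay it reads its state from the game instance's LevelsState array, indexed at three levels per section, and recolors its particle system to match.
; A W_Level_Point widget displays the labels, also refreshed during construction.
; SetIsActive toggles custom depth on the mesh; cursor and click events are empty, leaving level-opening logic disconnected.
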(event `self.ReceiveBeginPlay`
  (`self.UpdateText`)
  (`self.UpdateState` (`|GetArrayItem` (`/Game/Bluprints/Enemies/BP_KTWOPGameInstance.LevelsState` (cast `/Game/Bluprints/Enemies/BP_KTWOPGameInstance` (`GameplayStatics.GetGameInstance`) :!pure true)) (+ (- (`self.LevelNumber`) 1) (* (- (`self.LevelSection`) 1) 3)))))

(event `UpdateState`
  (params (State :type "/Game/Bluprints/Map/Tiles/WorldMap/E_Level_Point_Status Enum" :default "NewEnumerator0"))
  (bind _particlesystem (`self.ParticleSystem`))
  (bind _output_get (set `self.State` State))
  (switch `/Game/Bluprints/Map/Tiles/WorldMap/E_Level_Point_Status` _output_get
    (:`NewEnumerator0`
      (`ParticleSystemComponent.SetVectorParameter` _particlesystem "color" (`KismetMathLibrary.Conv_LinearColorToVector` (struct :`R` 15.0 :`B` 0.901959))))
    (:`NewEnumerator1`
      (`ParticleSystemComponent.SetVectorParameter` _particlesystem "color" (`KismetMathLibrary.Conv_LinearColorToVector` (struct))))
    (:`NewEnumerator2`
      (`ParticleSystemComponent.SetVectorParameter` _particlesystem "color" (`KismetMathLibrary.Conv_LinearColorToVector` (struct :`R` 0.5 :`G` 15.0 :`B` 0.100001))))))

(event `self.ueilcjiva_LOD4.OnBeginCursorOver`
  (params (TouchedComponent :type "PrimitiveComponent Object Reference")))

(event `self.ueilcjiva_LOD4.OnEndCursorOver`
  (params (TouchedComponent :type "PrimitiveComponent Object Reference")))

(event `self.ueilcjiva_LOD4.OnClicked`
  (params (TouchedComponent :type "PrimitiveComponent Object Reference") (ButtonPressed :type "Key Structure")))

(fn `SetIsActive`
  (params (IsActive :type Boolean))
  (`PrimitiveComponent.SetRenderCustomDepth` (`self.ueilcjiva_LOD4`) IsActive))

(fn `UpdateText`
  (`/Game/Bluprints/Map/Tiles/WorldMap/W_Level_Point.Update` (cast `/Game/Bluprints/Map/Tiles/WorldMap/W_Level_Point` (`WidgetComponent.GetWidget` (`self.Widget`)) :!pure true) (`self.LevelNumber`) (`self.LevelSection`)))

(fn `UserConstructionScript`
  (`self.UpdateText`))