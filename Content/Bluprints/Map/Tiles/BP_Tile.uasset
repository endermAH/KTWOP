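; BP_Tile is a map tile actor that keeps itself registered with the level's BP_Map and can hold one attached object.
; Its construction script finds the map, removes itself, runs the BPMapAnchorComponent's external construction step, then re-adds itself.
; DeleteFromEditor unregisters the tile from the map before destroying it.
; Helpers expose mesh and socket world locations, and Attach/Detach only store or clear a reference, without physical attachment.
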(fn `AddTileToMap`
  (params (Map :type "/Game/Bluprints/Map/BP_Map Object Reference"))
  (`/Game/Bluprints/Map/BP_Map.AddTile` Map self))

(fn `Attach`
  (params (Attached :type "Actor Object Reference"))
  (set `self.Attached` Attached))

(fn `DeleteFromEditor`
  (bind _returnvalue (`GameplayStatics.GetActorOfClass` "/Game/Bluprints/Map/BP_Map.BP_Map_C"))
  (`/Engine/EditorBlueprintResources/StandardMacros.IsValid` _returnvalue
    (:`Is Valid`
      (`/Game/Bluprints/Map/BP_Map.RemoveTile` _returnvalue self)
      (`self.K2_DestroyActor`))))

(fn `Detach`
  (returns (Detached :type "Actor Object Reference"))
  (locals (Temp :type "Actor Object Reference"))
  (set `local.Temp` (`self.Attached`))
  (set `self.Attached` null)
  (return (`local.Temp`)))

(fn `GetPosition`
  (returns (Position :type "Vector Structure"))
  (return (`SceneComponent.K2_GetComponentLocation` (`self.Mesh`))))

(fn `GetSocketPosition`
  (returns (Position :type "Vector Structure"))
  (return (`SceneComponent.K2_GetComponentLocation` (`self.Socket`))))

(fn `IsHasAttached`
  (returns (IsHasAttached :type Boolean))
  (return (`KismetSystemLibrary.IsValid` (`self.Attached`))))

(fn `RemoveTileFromMap`
  (params (Map :type "/Game/Bluprints/Map/BP_Map Object Reference"))
  (`/Game/Bluprints/Map/BP_Map.RemoveTile` Map self))

(fn `UserConstructionScript`
  (bind _returnvalue (`GameplayStatics.GetActorOfClass` "/Game/Bluprints/Map/BP_Map.BP_Map_C"))
  (`/Engine/EditorBlueprintResources/StandardMacros.IsValid` _returnvalue
    (:`Is Valid`
      (`self.RemoveTileFromMap` _returnvalue)
      (`/Game/Bluprints/Map/BP_MapAnchorComponent.ExternaConstructionScript` (`self.BP_MapAnchorComponent`))
      (`self.AddTileToMap` _returnvalue))))