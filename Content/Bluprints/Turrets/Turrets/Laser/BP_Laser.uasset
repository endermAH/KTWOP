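; Short-lived laser beam visual for turrets, drawn between a source positioned actor and an enemy target.
; Activate stores the view stats and plays a timeline that scales beam width toward the stats' laser width, while Update re-aims and stretches it between both actors and feeds endpoints to Niagara.
; The actor destroys itself when the timeline finishes or the initial actor checks fail; it applies no damage.
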(event `self.Activate`
  (params (ViewStats :type "LazerStats Structure (by ref)"))
  (bind _aspositioned_actor (cast `PositionedActor` (`self.TargetEnemy`) :!pure true))
  (bind _aspositioned_actor_2 (cast `PositionedActor` (`self.SorcePActor`) :!pure true))
  (bind _returnvalue (/ (`.LazerWidth` (break `LazerStats` (`self.Stats`))) 150.0))
  (set `self.Stats` ViewStats)
  (bind _asbase_enemy (cast `BaseEnemy` (`self.TargetEnemy`))
    (:`then`
      (bind _aspositioned_actor_3 (cast `PositionedActor` (`self.SorcePActor`))
        (:`then`
          (`/Engine/EditorBlueprintResources/StandardMacros.IsValid` _asbase_enemy
            (:`Is Valid`
              (`/Engine/EditorBlueprintResources/StandardMacros.IsValid` (`KismetSystemLibrary.Conv_InterfaceToObject` _aspositioned_actor_3)
                (:`Is Valid`
                  (bind _returnvalue_2 (`PositionedActor.GetLocation` _asbase_enemy))
                  (bind _returnvalue_3 (`PositionedActor.GetLocation` _aspositioned_actor_3))
                  (`self.Update` _returnvalue_2 _returnvalue_3)
                  (bind (_direction _alpha) (`Timeline|0-1-0`)
                    (:`Update`
                      (`SceneComponent.SetWorldScale3D` (`self.Scene`) (`KismetMathLibrary.VLerp` (`KismetMathLibrary.MakeVector` 0.0 0.0 (`self.Distance`)) (`KismetMathLibrary.MakeVector` _returnvalue _returnvalue (`self.Distance`)) _alpha))
                      (`/Engine/EditorBlueprintResources/StandardMacros.IsValid` (`KismetSystemLibrary.Conv_InterfaceToObject` _aspositioned_actor)
                        (:`Is Valid`
                          (bind _returnvalue_4 (`PositionedActor.GetLocation` _aspositioned_actor))
                          (`/Engine/EditorBlueprintResources/StandardMacros.IsValid` (`KismetSystemLibrary.Conv_InterfaceToObject` _aspositioned_actor_2)
                            (:`Is Valid`
                              (bind _returnvalue_5 (`PositionedActor.GetLocation` _aspositioned_actor_2))
                              (`self.Update` _returnvalue_5 _returnvalue_4))))))
                    (:`Finished`
                      (`self.K2_DestroyActor`))))
                (:`Is Not Valid`
                  (`self.K2_DestroyActor`))))
            (:`Is Not Valid`
              (`self.K2_DestroyActor`))))
        (:`CastFailed`
          (`self.K2_DestroyActor`))))
    (:`CastFailed`
      (`self.K2_DestroyActor`))))

(fn `Update`
  (params (From :type "Vector Structure") (To :type "Vector Structure"))
  (set `self.Distance` (/ (`KismetMathLibrary.VSize` (- (`local.To`) (`local.From`))) 254.0))
  (`SceneComponent.K2_SetWorldRotation` (`self.Scene`) (`KismetMathLibrary.ComposeRotators` (struct :`Pitch` 90.0) (`KismetMathLibrary.FindLookAtRotation` (`local.From`) (`local.To`))) false false)
  (`SceneComponent.K2_SetWorldLocation` (`self.Scene`) (`local.From`) false false)
  (`NiagaraComponent.SetVariableVec3` (`self.Niagara`) "User.BeamStart" (`local.From`))
  (`NiagaraComponent.SetVariableVec3` (`self.Niagara`) "User.BeamEnd" (`local.To`)))

(fn `UserConstructionScript`)