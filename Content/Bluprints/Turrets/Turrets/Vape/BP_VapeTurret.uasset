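; BP_VapeTurret is a turret Blueprint that fires a vape-style blast in sync with its animation.
; On BeginPlay it binds to the Shoot event of the Vape mesh's anim Blueprint, which activates the Blast component and calls RealShoot with zero delay.
; The EventShoot override is empty, leaving firing animation-driven, and an older delay-based shooting chain remains disconnected.
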(event `self.ReceiveBeginPlay`
  (bind _asbpa_vape_turret (cast `/Game/Bluprints/Turrets/Turrets/Vape/BPA_VapeTurret` (`SkeletalMeshComponent.GetAnimInstance` (`self.Vape`))))
  (add `/Game/Bluprints/Turrets/Turrets/Vape/BPA_VapeTurret.Shoot` _asbpa_vape_turret (delegate `OnShoot`)))

(event `OnShoot`
  (`ActorComponent.Activate` (`self.Blast`) true)
  (`Shootable.RealShoot` 0.0))

(event `self.EventShoot`
  (params (DeltaTime :type "Float (single-precision)")))

(fn `UserConstructionScript`)