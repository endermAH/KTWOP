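; BP_CannonBullet is the cannon turret's projectile, with ice, toxic and plasma visual variants.
; Each variant event reveals its matching component and sets the explosion color.
; On hitting a target it spawns a Niagara explosion tinted by that color, then destroys itself if no bounces remain in BaseStats.
; It also destroys itself when its travel distance is depleted.
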(event `self.ReceiveBeginPlay`)

(event `self.OnTargetHit`
  (params (OverlappedComponent :type "PrimitiveComponent Object Reference") (OtherActor :type "Actor Object Reference") (OtherComponent :type "PrimitiveComponent Object Reference") (OtherBodyIndex :type Integer) (bFromSweep :type Boolean) (Hit :type "HitResult Structure (by ref)"))
  (bind _basestats_bouncecount (break `BaseBulletStats` (`self.BaseStats`)))
  (bind _returnvalue (`NiagaraFunctionLibrary.SpawnSystemAtLocation` "/Game/Bluprints/Turrets/Particles/Explosion/NE_Explosion.NE_Explosion" (`self.K2_GetActorLocation`)))
  (`FXSystemComponent.SetColorParameter` _returnvalue "User.Color" (`self.ExplosionColor`))
  (if (<= _basestats_bouncecount 0)
    (`self.K2_DestroyActor`)))

(event `self.OnDistanceDeplete`
  (`self.K2_DestroyActor`))

(event `/Game/Bluprints/Turrets/Turrets/BPI_Projectile.IceOn`
  (`SceneComponent.SetVisibility` (`self.Icicle`) true false)
  (set `self.ExplosionColor` (struct :`G` 0.79842 :`B` 1.0 :`A` 1.0)))

(event `/Game/Bluprints/Turrets/Turrets/BPI_Projectile.ToxicOn`
  (`SceneComponent.SetVisibility` (`self.ToxicParticle`) true false)
  (set `self.ExplosionColor` (struct :`R` 0.323474 :`G` 1.0 :`A` 1.0)))

(event `/Game/Bluprints/Turrets/Turrets/BPI_Projectile.PlasmaOn`
  (`SceneComponent.SetVisibility` (`self.PlasmaParitcle`) true false)
  (set `self.ExplosionColor` (struct :`R` 1.0 :`B` 0.995726 :`A` 1.0)))

(fn `UserConstructionScript`)