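; Cannon turret that fires with an animation, Niagara muzzle effect, random sound and an inherited RealShoot call.
; EventShoot uses a Gate that closes after each shot and reopens after the modified ShootDelay.
; Construction fills Statuses with copies of the base and plasma damage statuses.
; Ice, toxic and plasma events recolor the muzzle effect and an emissive dynamic material created at BeginPlay.
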(event `self.ReceiveBeginPlay`
  (`self.CreateDMIs`))

(event `self.EventShoot`
  (params (DeltaTime :type "Float (single-precision)"))
  (`/Engine/EditorBlueprintResources/StandardMacros.Gate` false :!label _label
    (:`Exit`
      (`SkeletalMeshComponent.PlayAnimation` (`self.SkeletalMesh`) "/Game/Bluprints/Turrets/Meshes/Cannon/Cannon_Anim.Cannon_Anim" false)
      (`ActorComponent.Activate` (`self.Muzzle`) true)
      (`GameplayStatics.PlaySoundAtLocation` "/Game/Sounds/Cannon/Cues/RandomCannonShot.RandomCannonShot" (`SceneComponent.K2_GetComponentLocation` (`self.ArrowComponent`)) (struct) 1.0 1.0 0.0 null null null null)
      (`Shootable.RealShoot` 1000.0)
      (`|ExecutionSequence`
        (:`then_0`
          (goto _label :!via `Close`))
        (:`then_1`
          (`KismetSystemLibrary.Delay` (`.ShootDelay` (break `BaseTurretStats` (`self.ModifiedStats`))))
          (goto _label :!via `Open`))))))

(event `/Game/Bluprints/Turrets/Turrets/BPI_Elementable.IceOn`
  (`self.SetMuzzleColor` (struct :`R` 0.7 :`G` 5.6 :`B` 37.0 :`A` 1.0))
  (`self.SetColor` (struct :`G` 0.6 :`B` 1.0 :`A` 1.0)))

(event `/Game/Bluprints/Turrets/Turrets/BPI_Elementable.ToxicOn`
  (`self.SetMuzzleColor` (struct :`R` 5.6 :`G` 37.0 :`B` 0.7 :`A` 1.0))
  (`self.SetColor` (struct :`G` 1.0 :`A` 1.0)))

(event `/Game/Bluprints/Turrets/Turrets/BPI_Elementable.PlasmaOn`
  (`self.SetMuzzleColor` (struct :`R` 37.0 :`G` 5.6 :`B` 37.0 :`A` 1.0))
  (`self.SetColor` (struct :`R` 1.0 :`B` 1.0 :`A` 1.0)))

(fn `CreateDMIs`
  (bind _returnvalue (`PrimitiveComponent.CreateDynamicMaterialInstance` (`self.SkeletalMesh`) 1 "/Game/Bluprints/Turrets/Materials/MI_EmmissiveTurret.MI_EmmissiveTurret" "None"))
  (set `self.DMI` _returnvalue))

(fn `SetColor`
  (params (Color :type "LinearColor Structure"))
  (`MaterialInstanceDynamic.SetVectorParameterValue` (`self.DMI`) "Color" Color))

(fn `SetMuzzleColor`
  (params (Color :type "LinearColor Structure"))
  (`FXSystemComponent.SetColorParameter` (`self.Muzzle`) "User.Color" Color))

(fn `UserConstructionScript`
  (`|ExecutionSequence`
    (:`then_0`
      (bind _returnvalue (`BaseStatus.MakeStatusCopy` :`self` (`/Game/Bluprints/StatusesHolder.BaseDmg` (`self.StatusesHolder`)) :`outer` self)))
    (:`then_1`
      (bind _returnvalue_2 (`BaseStatus.MakeStatusCopy` :`self` (`/Game/Bluprints/StatusesHolder.PlasmaDMG` (`self.StatusesHolder`)) :`outer` self)))
    (:`then_2`
      (set `self.Statuses` (`|MakeArray` _returnvalue _returnvalue_2)))))