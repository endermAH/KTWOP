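; Cannon turret Blueprint that fires after a delay and carries base and plasma damage statuses.
; The shoot event waits for the base-stat shoot delay, then calls RealShoot.
; The construction script copies both statuses from StatusesHolder, owned by the turret, into its Statuses array.
; Animation playback, rock-module setup and a modified-stat firing delay are present but unconnected.
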(event `self.ReceiveBeginPlay`)

(event `self.ReceiveTick`
  (params (DeltaSeconds :type "Float (single-precision)")))

(event `self.EventShoot`
  (params (DeltaTime :type "Float (single-precision)"))
  (`KismetSystemLibrary.Delay` (`.ShootDelay` (break `BaseTurretStats` (`self.BaseStats`))))
  (`Shootable.RealShoot` 1000.0))

(fn `UserConstructionScript`
  (`|ExecutionSequence`
    (:`then_0`
      (bind _returnvalue (`BaseStatus.MakeStatusCopy` :`self` (`/Game/Bluprints/StatusesHolder.BaseDmg` (`self.StatusesHolder`)) :`outer` self)))
    (:`then_1`
      (bind _returnvalue_2 (`BaseStatus.MakeStatusCopy` :`self` (`/Game/Bluprints/StatusesHolder.PlasmaDMG` (`self.StatusesHolder`)) :`outer` self)))
    (:`then_2`
      (set `self.Statuses` (`|MakeArray` _returnvalue _returnvalue_2)))))