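; BP_VapeTurret is a turret Blueprint whose firing is driven by the animation Blueprint of its Vape mesh.
; On BeginPlay it casts that mesh's anim instance to BPA_VapeTurret and registers OnShoot as its shoot callback, which then calls RealShoot.
; EventShoot is left empty, and an older delay-based firing chain using ShootDelay remains disconnected.
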(event `self.ReceiveBeginPlay`
  (bind _asbpa_vape_turret (cast `/Game/Bluprints/Turrets/BPA_VapeTurret` (`SkeletalMeshComponent.GetAnimInstance` (`self.Vape`))))
  (add `/Game/Bluprints/Turrets/BPA_VapeTurret.Shoot` _asbpa_vape_turret (delegate `OnShoot`)))

(event `OnShoot`
  (`Shootable.RealShoot` 0.0))

(event `self.EventShoot`
  (params (DeltaTime :type "Float (single-precision)")))

(fn `UserConstructionScript`)