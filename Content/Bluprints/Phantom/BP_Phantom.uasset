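; BP_Phantom is a turret placement preview that shows whether a tile can be built on and spawns the turret there.
; Construction creates a dynamic material on the Phantom component, which Update tints green over Obstacle tiles and red over Path tiles.
; TrySpawn accepts only Obstacle tiles with nothing attached, spawns TurretClass at the tile's socket, attaches it and reports success.
; The preview color ignores whether a tile is already occupied.
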(fn `Disable`
  (`MaterialInstanceDynamic.SetVectorParameterValue` (`self.MI`) "Color" (make `LinearColor` 1.0 0.0 0.0 1.0)))

(fn `Enable`
  (`MaterialInstanceDynamic.SetVectorParameterValue` (`self.MI`) "Color" (make `LinearColor` 0.0 1.0 0.0 1.0)))

(fn `TrySpawn`
  (params (Tile :type "/Game/Bluprints/Map/Tiles/BP_Tile Object Reference"))
  (returns (IsSpawned :type Boolean))
  (if (`|EnumEquality` (`/Game/Bluprints/Map/Tiles/BP_Tile.Type` (`local.Tile`)) "NewEnumerator0")
    (bind _ishasattached (`/Game/Bluprints/Map/Tiles/BP_Tile.IsHasAttached` (`local.Tile`)))
    (if (not _ishasattached)
      (bind _position (`/Game/Bluprints/Map/Tiles/BP_Tile.GetSocketPosition` (`local.Tile`)))
      (bind _returnvalue (`|SpawnActorFromClass` (`self.TurretClass`) (`KismetMathLibrary.MakeTransform` _position) "Undefined" "OverrideRootScale" null null))
      (`/Game/Bluprints/Map/Tiles/BP_Tile.Attach` (`local.Tile`) _returnvalue)
      (return true)
      (else
        (return false)))
    (else
      (return false))))

(fn `Update`
  (params (Tile :type "/Game/Bluprints/Map/Tiles/BP_Tile Object Reference"))
  (returns (IsCanSpawn :type Boolean))
  (switch `/Game/Bluprints/Map/E_TileType` (`/Game/Bluprints/Map/Tiles/BP_Tile.Type` Tile)
    (:`NewEnumerator0`
      (`self.Enable`)
      (return true))
    (:`NewEnumerator1`
      (`self.Disable`)
      (return false))))

(fn `UserConstructionScript`
  (bind _returnvalue (`PrimitiveComponent.CreateDynamicMaterialInstance` (`self.Phantom`) 0 null "None"))
  (set `self.MI` _returnvalue))